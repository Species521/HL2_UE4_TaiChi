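; Taichi character Blueprint with a skeletal mesh and leftover, mostly unfinished animation control logic.
; A custom event clears the AnimPause flag and stops the mesh's animation when that flag is set.
; Tick checks AnimStart but does nothing, while the nodes that play the Taichi animation once are disconnected and never run.
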(event Custom|CustomEvent
  (params (DeltaSeconds :type Float%20%28single-precision%29))
  (if (Variables|Default|GetanimPause)
    (Variables|Default|SetanimPause false)
    (Audio|Components|Audio|Stop (Variables|Default|Gettaichi_skelmesh))))

(event EventBeginPlay)

(event Collision|EventActorBeginOverlap
  (params (OtherActor :type Actor%20Object%20Reference)))

(event EventTick
  (params (DeltaSeconds :type Float%20%28single-precision%29))
  (if (Variables|Default|GetanimStart)
    _))

(fn ConstructionScript)